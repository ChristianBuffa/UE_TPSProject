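; BP_Cover is a cover actor for enemies that supplies the cover position farthest from the player.
; GetAllSockets adds the actor's location to each SocketsValues offset, ignoring rotation, and appends the results to SocketPositions without clearing it.
; GetOptimalSocket scans those positions, keeps the one with the greatest distance to player character 0, prints it and returns it.
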(fn `GetAllSockets`
  (returns (SceneComponents :type "Array of Vector Structure"))
  (bind _socketpositions (`self.SocketPositions`))
  (for _array_element (`self.SocketsValues`)
    (`KismetArrayLibrary.Array_Add` _socketpositions (+ _array_element (`self.K2_GetActorLocation` self))))
  (return _socketpositions))

(fn `GetOptimalSocket`
  (returns (OptimalSocket :type "Vector Structure"))
  (bind _previousdistance (`self.PreviousDistance`))
  (bind _optimalsocket (`self.OptimalSocket`))
  (bind _scenecomponents (`self.GetAllSockets`))
  (for _array_element _scenecomponents
    (if (<= _previousdistance 0.0)
      (bind _returnvalue (`KismetMathLibrary.Vector_Distance` _array_element (`self.K2_GetActorLocation` (`GameplayStatics.GetPlayerCharacter` 0))))
      (set `self.PreviousDistance` _returnvalue :!label _label)
      (set `self.OptimalSocket` _array_element)
      (elif (> _returnvalue _previousdistance)
        (goto _label))))
  (set `self.PreviousDistance` 0.0)
  (`KismetSystemLibrary.PrintString` (`KismetStringLibrary.Conv_VectorToString` _optimalsocket))
  (return _optimalsocket))

(fn `UserConstructionScript`)